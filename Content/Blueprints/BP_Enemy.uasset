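; BP_Enemy is an enemy that chases and attacks the player, with a floating health bar.
; Detection overlap starts a self-repeating AI MoveTo, while a looping delay from BeginPlay triggers montage attacks within AttackRadius.
; Attack damage lands after a delay, without rechecking range.
; Damage spawns Niagara effects and ragdolls the enemy at zero health; Tick turns and updates the health widget.
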(event OnComponentBeginOverlap(DetectionRadius)
  (params (OverlappedComponent :type Primitive%20Component%20Object%20Reference) (OtherActor :type Actor%20Object%20Reference) (OtherComp :type Primitive%20Component%20Object%20Reference) (OtherBodyIndex :type Integer) (bFromSweep :type Boolean) (SweepResult :type Hit%20Result%20Structure%20%28by%20ref%29))
  (Utilities|Casting|CastToBP_ThirdPersonCharacter OtherActor)
  (CallFunction|ChasePlayer))

(event OnComponentBeginOverlap(AttackRadius)
  (params (OverlappedComponent :type Primitive%20Component%20Object%20Reference) (OtherActor :type Actor%20Object%20Reference) (OtherComp :type Primitive%20Component%20Object%20Reference) (OtherBodyIndex :type Integer) (bFromSweep :type Boolean) (SweepResult :type Hit%20Result%20Structure%20%28by%20ref%29))
  ;[1 1 1] Атака игрока
  (Utilities|Casting|CastToBP_ThirdPersonCharacter OtherActor)
  (Variables|Default|SetIsInRadius true))

(event OnComponentEndOverlap(AttackRadius)
  (params (OverlappedComponent :type Primitive%20Component%20Object%20Reference) (OtherActor :type Actor%20Object%20Reference) (OtherComp :type Primitive%20Component%20Object%20Reference) (OtherBodyIndex :type Integer))
  ;[1 1 1] Атака игрока
  (Utilities|Casting|CastToBP_ThirdPersonCharacter OtherActor)
  (Variables|Default|SetIsInRadius false))

(event Custom|Chase%20Player
  (if (not (Variables|Default|GetIsDead))
    (AI|AIMoveTo self "0, 0, 0" (Game|GetPlayerCharacter 0) 1.2e+02 false
      (:OnSuccess
        (CallFunction|ChasePlayer)))))

(event Custom|Attack%20Player
  ;[1 1 1] Атака игрока
  (if (Variables|Default|GetIsInRadius)
    (if (not (Variables|Default|GetIsDead))
      (Animation|PlayAnimMontage "/Game/Enemy_Animations/Fire_Shotgun_Hip_Montage.Fire_Shotgun_Hip_Montage" 1.0 "None")
      (Utilities|FlowControl|Delay 1.0)
      (bind _asbp_third_person_character (Utilities|Casting|CastToBP_ThirdPersonCharacter (Game|GetPlayerCharacter 0)))
      (Game|Damage|ApplyDamage _asbp_third_person_character 1e+01 0 0))))

(event Game|Damage|EventAnyDamage
  (params (Damage :type Float%20%28single-precision%29) (DamageType :type Damage%20Type%20Object%20Reference) (InstigatedBy :type Controller%20Object%20Reference) (DamageCauser :type Actor%20Object%20Reference))
  (Variables|Default|SetHealth (- (Variables|Default|GetHealth) Damage))
  (Niagara|SpawnSystematLocation "/Game/NiagaraSystem/NS_Damage.NS_Damage" (Transformation|GetActorLocation) "0, 0, 0" "1.000000,1.000000,1.000000" true true "AutoRelease")
  (if (<= (Variables|Default|GetHealth) 0.0)
    (Physics|SetSimulatePhysics (Variables|Character|GetMesh) true)
    (Components|Movement|StopMovementImmediately (Variables|Character|GetCharacterMovement))
    (Variables|Default|SetIsDead true)))

(event EventBeginPlay
  (Utilities|FlowControl|RetriggerableDelay 1.0 :!label _label)
  (CallFunction|AttackPlayer)
  (goto _label))

(event EventTick
  (params (DeltaSeconds :type Float%20%28single-precision%29))
  (Transformation|SetWorldRotation (Variables|Default|GetHealth%20Widget) (Math|Rotator|FindLookatRotation (Transformation|GetWorldLocation (Variables|Default|GetHealth%20Widget)) (Transformation|GetActorLocation (Game|GetPlayerCharacter 0))) false false)
  (bind _aswb_enemy_health_bar (Utilities|Casting|CastToWB_EnemyHealthBar (UserInterface|GetWidget (Variables|Default|GetHealth%20Widget))))
  (Progress|SetPercent (Variables|/Game/UI/WB_EnemyHealthBar.WB_EnemyHealthBar_C|GetHealth _aswb_enemy_health_bar) (/ (Variables|Default|GetHealth) 5e+01)))

(fn ConstructionScript)